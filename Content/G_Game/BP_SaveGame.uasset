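; BP_SaveGame is a SaveGame Blueprint meant to persist an array of player results in the "PlayerResultSlot" slot.
; LoadData checks that the slot exists, loads it and copies the saved ResultArray into this instance.
; SaveData writes a newly created, unmodified save object to the slot, so its parameter is not saved; the node appending it to ResultArray is disconnected.
; NewFunction is an empty stub.
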(fn NewFunction)

(fn SaveData
  (params (NewParam :type Player%20Result%20Structure))
  (bind _returnvalue (SaveGame|CreateSaveGameObject "BP_SaveGame_C"))
  (SaveGame|SaveGametoSlot _returnvalue "PlayerResultSlot"))

(fn LoadData
  (bind _returnvalue (SaveGame|DoesSaveGameExist "PlayerResultSlot"))
  (if _returnvalue
    (bind _returnvalue_2 (SaveGame|LoadGamefromSlot "PlayerResultSlot"))
    (bind _asbp_save_game (Utilities|Casting|CastToBP_SaveGame _returnvalue_2))
    (Variables|Default|SetResultArray (Variables|BP_SaveGame_C|GetResultArray _asbp_save_game))))