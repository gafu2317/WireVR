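; Spectator manager that gives the other players' VR pawns their own spectator cameras.
; AddCamera gathers all VRPawn actors, removes the locally controlled one, and spawns a BP_SpectatorCamera for each remaining pawn.
; Each camera receives one of three player render targets by index and attaches to its pawn, using an offset along the pawn's negative forward vector as relative location.
; Spawned cameras are stored in SpectatorCameras.
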(event Custom|AddCamera
  (bind _output_get (Variables|Default|SetRenderTargets (Utilities|Array|MakeArray "/Game/K_Level/Spectator/RT_Player1.RT_Player1" "/Game/K_Level/Spectator/RT_Player2.RT_Player2" "/Game/K_Level/Spectator/RT_Player3.RT_Player3")))
  (bind _outactors (Actor|GetAllActorsOfClass "/Script/VRTemplate.VRPawn"))
  (bind _output_get_2 (Variables|Default|SetPlayers _outactors))
  (for (_array_element _array_index) _output_get_2
    (if (== _array_element (Pawn|GetControlledPawn (Game|GetPlayerController 0)))
      (Utilities|Array|RemoveIndex (Variables|Default|GetPlayers) _array_index)))
  (for (_array_element_2 _array_index_2) _output_get_2
    (bind _output_get_3 (Variables|Default|SetTargetPawn _array_element_2))
    (bind _returnvalue (Game|SpawnActorfromClass "/Game/K_Level/Spectator/BP_SpectatorCamera.BP_SpectatorCamera_C" (Math|Transform|MakeTransform (* (Transformation|GetActorForwardVector _output_get_3) -3e+02)) "Undefined" "MultiplyWithRoot" 0 (Utilities|Array|Get(acopy) _output_get _array_index_2) 0))
    (Transformation|AttachActorToActor _returnvalue (Variables|Default|GetTargetPawn) "None" "KeepRelative" "KeepRelative" "KeepRelative" false)
    (Utilities|Array|Add (Variables|Default|GetSpectatorCameras) _returnvalue)))

(event Collision|EventActorBeginOverlap
  (params (OtherActor :type Actor%20Object%20Reference)))

(event EventTick
  (params (DeltaSeconds :type Float%20%28single-precision%29)))

(fn ConstructionScript)