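; Player character Blueprint, named for wire-based play, that adds the crosshair HUD and a test reset, with no wire logic in its own graphs.
; On BeginPlay it creates WBP_Crosshair, adds it to the viewport and passes its Crosshair element to SetCrosshairWidget.
; Holding the TestReset input for over three seconds moves the character to the world origin, with IsReset limiting this to once per press.
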(event Input|EnhancedActionEvents|EnhancedInputActionTestReset
  (params (ActionValue :type Boolean) (ElapsedSeconds :type Float%20%28double-precision%29) (TriggeredSeconds :type Float%20%28double-precision%29) (InputAction :type Input%20Action%20Object%20Reference :default "/Game/S_Player/TestReset.TestReset"))
  (:Triggered
    (if (> ElapsedSeconds 3.0)
      (if (not (Variables|Default|GetisReset))
        (Transformation|SetActorLocation "0, 0, 0" false false)
        (Variables|Default|SetisReset true))))
  (:Started
    (Variables|Default|SetisReset false)))

(event EventBeginPlay
  (bind _returnvalue (UserInterface|CreateWidget "/Game/S_Player/WBP_Crosshair.WBP_Crosshair_C"))
  (UserInterface|Viewport|AddtoViewport _returnvalue 0)
  (Class|WireCharacter|SetCrosshairWidget (Variables|/Game/S_Player/WBP_Crosshair.WBP_Crosshair_C|GetCrosshair _returnvalue)))

(event Collision|EventActorBeginOverlap
  (params (OtherActor :type Actor%20Object%20Reference)))

(event EventTick
  (params (DeltaSeconds :type Float%20%28single-precision%29)))

(fn ConstructionScript)