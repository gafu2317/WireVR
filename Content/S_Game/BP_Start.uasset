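; BP_Start is an enclosure of ceiling, floor and four wall components that can be removed, likely a start-area box.
; Removal turns off collision and hides each of the six pieces in sequence.
; BeginPlay runs it only on the server, while the Start event runs the same chain without that check.
; Nothing in the graph restores the pieces.
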(event Custom|Start
  (bind _ceiling (Variables|Default|GetCeiling))
  (bind _floor (Variables|Default|GetFloor))
  (bind _wall_f (Variables|Default|GetWall_F))
  (bind _wall_r (Variables|Default|GetWall_R))
  (bind _wall_l (Variables|Default|GetWall_L))
  (bind _wall_b (Variables|Default|GetWall_B))
  (Collision|SetCollisionEnabled _ceiling "NoCollision")
  (Rendering|SetVisibility _ceiling false false)
  (Collision|SetCollisionEnabled _floor "NoCollision")
  (Rendering|SetVisibility _floor false false)
  (Collision|SetCollisionEnabled _wall_f "NoCollision")
  (Rendering|SetVisibility _wall_f false false)
  (Collision|SetCollisionEnabled _wall_r "NoCollision")
  (Rendering|SetVisibility _wall_r false false)
  (Collision|SetCollisionEnabled _wall_l "NoCollision")
  (Rendering|SetVisibility _wall_l false false)
  (Collision|SetCollisionEnabled _wall_b "NoCollision")
  (Rendering|SetVisibility _wall_b false false))

(event EventBeginPlay
  (bind _ceiling (Variables|Default|GetCeiling))
  (bind _floor (Variables|Default|GetFloor))
  (bind _wall_f (Variables|Default|GetWall_F))
  (bind _wall_r (Variables|Default|GetWall_R))
  (bind _wall_l (Variables|Default|GetWall_L))
  (bind _wall_b (Variables|Default|GetWall_B))
  (if (Networking|IsServer)
    (Collision|SetCollisionEnabled _ceiling "NoCollision")
    (Rendering|SetVisibility _ceiling false false)
    (Collision|SetCollisionEnabled _floor "NoCollision")
    (Rendering|SetVisibility _floor false false)
    (Collision|SetCollisionEnabled _wall_f "NoCollision")
    (Rendering|SetVisibility _wall_f false false)
    (Collision|SetCollisionEnabled _wall_r "NoCollision")
    (Rendering|SetVisibility _wall_r false false)
    (Collision|SetCollisionEnabled _wall_l "NoCollision")
    (Rendering|SetVisibility _wall_l false false)
    (Collision|SetCollisionEnabled _wall_b "NoCollision")
    (Rendering|SetVisibility _wall_b false false)))

(fn ConstructionScript)