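; Course manager for the VR race that registers itself on the local player's PlayerState shortly after BeginPlay.
; RaceSetup moves the goal, toggles the course-switch wall for the selected race and starts the BGM.
; Lookup functions map player IDs 2–4 to start or practice markers.
; The respawn floor teleports the local VR pawn (on clients or a solo server) to its start, always using the default course.
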(event OnComponentBeginOverlap(RespornFloor)
  (params (OverlappedComponent :type Primitive%20Component%20Object%20Reference) (OtherActor :type Actor%20Object%20Reference) (OtherComp :type Primitive%20Component%20Object%20Reference) (OtherBodyIndex :type Integer) (bFromSweep :type Boolean) (SweepResult :type Hit%20Result%20Structure%20%28by%20ref%29))
  (bind _asbp_player_controller_vr (Utilities|Casting|CastToBP_PlayerControllerVR (Components|GetOwner OtherActor)))
  (if (Pawn|IsLocalPlayerController _asbp_player_controller_vr)
    (if (Networking|IsServer)
      (if (Variables|/Game/G_Game/BP_GameInstance.BP_GameInstance_C|GetisSolo (.AsBP%20Game%20Instance (Utilities|Casting|CastToBP_GameInstance (Game|GetGameInstance))))
        (bind _startposition (CallFunction|GetStartPosition 0 (Variables|/Game/S_Game/BP_PlayerStateVR.BP_PlayerStateVR_C|GetID (.AsBP%20Player%20State%20VR (Utilities|Casting|CastToBP_PlayerStateVR (Variables|/Script/Engine.Controller|GetPlayerState _asbp_player_controller_vr)))) :!label _label))
        (Class|VRPawn|SetPosition (.AsVRPawn (Utilities|Casting|CastToVRPawn (Pawn|GetControlledPawn _asbp_player_controller_vr))) _startposition))
      (else
        (goto _label)))))

(event Custom|Race%20Setup
  (params (RaceNumber :type Integer))
  (bind _returnvalue (== RaceNumber 2))
  (bind _courseswitchwall (Variables|Default|GetCourseSwitchWall))
  (bind _bp_goal (Variables|Default|GetBP_Goal))
  (bind _returnvalue_2 (not _returnvalue))
  (if _returnvalue
    (Transformation|SetWorldLocation _bp_goal (Transformation|GetWorldLocation (Variables|Default|GetGoal2)) false false)
    (else
      (Transformation|SetWorldLocation _bp_goal (Transformation|GetWorldLocation (Variables|Default|GetGoal1)) false false)))
  (Collision|SetActorEnableCollision _courseswitchwall _returnvalue_2)
  (Rendering|SetVisibility (Variables|/Script/Engine.StaticMeshActor|GetStaticMeshComponent _courseswitchwall) _returnvalue_2 false)
  (Audio|Components|Audio|Play (Variables|Default|GetBGM) 0.0))

(event EventBeginPlay
  ;[0.15 0.15 0.15 0.5] コースに遷移してきたらPlayerStateに情報を登録
  (Utilities|FlowControl|Delay 1.0)
  (bind _asbp_player_controller_vr (Utilities|Casting|CastToBP_PlayerControllerVR (Game|GetPlayerController 0)))
  (bind _asbp_player_state_vr (Utilities|Casting|CastToBP_PlayerStateVR (Variables|/Script/Engine.Controller|GetPlayerState _asbp_player_controller_vr)))
  (Variables|/Game/S_Game/BP_PlayerStateVR.BP_PlayerStateVR_C|SetCourseManager _asbp_player_state_vr self))

(fn ConstructionScript)

(fn GetStartPosition
  (params (RaceNumber :type Integer) (playerIndex :type Integer))
  (if (== RaceNumber 2)
    (switch int playerIndex
      (:Default
        _)
      (:0
        _)
      (:1
        _)
      (:2
        (return (Transformation|GetWorldLocation (Variables|Default|GetStart2_01))))
      (:3
        (return (Transformation|GetWorldLocation (Variables|Default|GetStart2_02))))
      (:4
        (return (Transformation|GetWorldLocation (Variables|Default|GetStart2_03)))))
    (return "0, 0, 0")
    (else
      (switch int playerIndex
        (:Default
          _)
        (:0
          _)
        (:1
          _)
        (:2
          (return (Transformation|GetWorldLocation (Variables|Default|GetStart1_01))))
        (:3
          (return (Transformation|GetWorldLocation (Variables|Default|GetStart1_02))))
        (:4
          (return (Transformation|GetWorldLocation (Variables|Default|GetStart1_03)))))
      (return "0, 0, 0"))))

(fn GetPracticePosition
  (params (PlayerIndex :type Integer))
  (switch int PlayerIndex
    (:Default
      _)
    (:0
      _)
    (:1
      _)
    (:2
      (return (Transformation|GetWorldLocation (Variables|Default|GetPractice01))))
    (:3
      (return (Transformation|GetWorldLocation (Variables|Default|GetPractice02))))
    (:4
      (return (Transformation|GetWorldLocation (Variables|Default|GetPractice03)))))
  (return "0, 0, 0"))