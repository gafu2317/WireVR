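; BP_GameManager runs the race flow: host-side player registration, race timing, goal UI and the top-three result display.
; RaceStart stamps the start time, and RaceEnd, fired by the Goal actor, passes elapsed time to MakeRaceResult.
; Once all players finish, SaveRaceResult copies to PlayerResults and clears RaceResults before DisplayRanking reads that same array.
; MakeRaceRanking bubble-sorts by time but is not called here.
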(event Custom|Race%20Start
  (Variables|Default|SetStartTime (Math|DateTime|Now))
  (Variables|Default|SetisGoal false)
  (CallFunction|ShowTimer))

(event Custom|Race%20End
  (bind _wbp_goal (Variables|Default|GetWBP_Goal))
  (if (!= (Variables|Default|GetisGoal) true)
    (Variables|Default|SetisGoal true)
    (bind _output_get (Variables|Default|SetRaceTime (- (Math|DateTime|Now) (Variables|Default|GetStartTime))))
    (CallFunction|MakeRaceResult (Variables|Default|GetPlayerId) _output_get)
    (UserInterface|Animation|PlayAnimation _wbp_goal (Variables|/Game/K_Level/WBP_Goal.WBP_Goal_C|GetGoal _wbp_goal) 0.0 1 "Forward" 1.0 false)
    (Widget|SetVisibility _wbp_goal "Visible")
    (Default|StartBlinking (Variables|Default|GetWBP_Timer))
    (Development|PrintString 0 (Utilities|String|ToString(Text) (Class|KismetTextLibrary|AsTimespanTimespan _output_get)))))

(event Custom|Make%20Race%20Result
  (params (PlayerId :type Integer) (RaceTime :type Timespan%20Structure))
  (bind _raceresults (Variables|Default|GetRaceResults))
  ;[0.15 0.15 0.15 0.5] レース結果集計
  (bind (_array_element _array_index) (Utilities|Array|ForEachLoopwithBreak _raceresults :!label _label)
    (:LoopBody
      (if (== (.PlayerId (Utilities|Struct|BreakRaceResult _array_element)) PlayerId)
        (Utilities|Struct|SetmembersinRaceResult (Utilities|Array|Get(acopy) _raceresults _array_index) RaceTime)
        (bind _result (Math|Integer|IncrementInt (Variables|Default|GetGoalCount))
          (:%20%20
            (Variables|Default|SetGoalCount _result)
            (goto _label Break)))))
    (:Completed
      ;[0.15 0.15 0.15 0.5] 全員がゴールした場合
      (if (== (Variables|Default|GetGoalCount) (Utilities|Array|Length (Variables|Default|GetRaceResults)))
        (CallFunction|SaveRaceResult)
        (CallFunction|DisplayRanking)
        (Variables|Default|SetGoalCount 0)))))

(event Custom|Save%20Race%20Result
  (bind _raceresults (Variables|Default|GetRaceResults))
  (for _array_element _raceresults
    (Utilities|Array|Add (Variables|Default|GetPlayerResults) (Utilities|Struct|MakePlayerResult (.PlayerName (Utilities|Struct|BreakRaceResult _array_element)) (.RaceTime (Utilities|Struct|BreakRaceResult _array_element)))))
  (Utilities|Array|Clear _raceresults))

(event Custom|Register%20Player
  (params (DeviceId :type Integer) (PlayerName :type String) (SkinId :type Integer))
  (bind _raceresults (Variables|Default|GetRaceResults))
  (bind _returnvalue (Utilities|Array|Length _raceresults))
  (if (Variables|/Game/G_Game/BP_GameInstance.BP_GameInstance_C|GetIsServer (Variables|Default|GetGameInstance))
    (Utilities|Array|Add _raceresults (Utilities|Struct|MakeRaceResult PlayerName _returnvalue "+00000000.00:00:00.000000000"))
    (Default|SetPlayerIdHost (Variables|Default|GetPlayerController) DeviceId _returnvalue)))

(event Custom|Display%20Ranking
  (bind _wbp_raceresult (Variables|Default|GetWBP_RaceResult))
  (bind _raceresults (Variables|Default|GetRaceResults))
  (bind _output (Utilities|Array|Get(acopy) _raceresults 2))
  (bind _output_2 (Utilities|Array|Get(acopy) _raceresults))
  (bind _output_3 (Utilities|Array|Get(acopy) _raceresults 1))
  (bind (_playername _playerid _racetime) (Utilities|Struct|BreakRaceResult _output))
  (bind (_playername_2 _playerid_2 _racetime_2) (Utilities|Struct|BreakRaceResult _output_2))
  (bind (_playername_3 _playerid_3 _racetime_3) (Utilities|Struct|BreakRaceResult _output_3))
  (Rendering|Components|TextRender|SetText (Variables|/Game/K_Level/WBP_RaceResult.WBP_RaceResult_C|GetPlayer_1st _wbp_raceresult) (Utilities|Text|ToText(String) (Utilities|String|Append "1位　" _playername_2)))
  (bind _timestring (CallFunction|TimespantoString _racetime_2))
  (Rendering|Components|TextRender|SetText (Variables|/Game/K_Level/WBP_RaceResult.WBP_RaceResult_C|GetTime_1st _wbp_raceresult) (Utilities|Text|ToText(String) _timestring))
  (if (== (Utilities|Array|Length (Variables|Default|GetRaceResults)) 1)
    _
    (else
      (Rendering|Components|TextRender|SetText (Variables|/Game/K_Level/WBP_RaceResult.WBP_RaceResult_C|GetPlayer_2nd _wbp_raceresult) (Utilities|Text|ToText(String) (Utilities|String|Append "2位　" _playername_3)))
      (bind _timestring_2 (CallFunction|TimespantoString _racetime_3))
      (Rendering|Components|TextRender|SetText (Variables|/Game/K_Level/WBP_RaceResult.WBP_RaceResult_C|GetTime_2nd _wbp_raceresult) (Utilities|Text|ToText(String) _timestring_2))
      (if (== (Utilities|Array|Length (Variables|Default|GetRaceResults)) 2)
        _
        (else
          (Rendering|Components|TextRender|SetText (Variables|/Game/K_Level/WBP_RaceResult.WBP_RaceResult_C|GetPlayer_3rd _wbp_raceresult) (Utilities|Text|ToText(String) (Utilities|String|Append "3位　" _playername)))
          (bind _timestring_3 (CallFunction|TimespantoString _racetime))
          (Rendering|Components|TextRender|SetText (Variables|/Game/K_Level/WBP_RaceResult.WBP_RaceResult_C|GetTime_3rd _wbp_raceresult) (Utilities|Text|ToText(String) _timestring_3))))))
  (UserInterface|Animation|PlayAnimation _wbp_raceresult (Variables|/Game/K_Level/WBP_RaceResult.WBP_RaceResult_C|GetShow _wbp_raceresult) 0.0 1 "Forward" 1.0 false)
  (Widget|SetVisibility _wbp_raceresult "HitTestInvisible"))

(event Custom|Make%20Race%20Ranking
  (bind _raceresults (Variables|Default|GetRaceResults))
  (bind _raceresults_2 (Variables|Default|GetRaceResults))
  (bind _returnvalue (Utilities|Array|Length _raceresults))
  ;[0.15 0.15 0.15 0.5] レース結果をタイム順に並べ替え
  (for _index (range 0 (- _returnvalue 1))
    (for _index_2 (range 0 (- _returnvalue 2))
      (if (> (.RaceTime (Utilities|Struct|BreakRaceResult (Utilities|Array|Get(acopy) _raceresults_2 _index_2))) (.RaceTime (Utilities|Struct|BreakRaceResult (Utilities|Array|Get(acopy) _raceresults_2 (+ _index_2 1)))))
        (Utilities|Array|Swap _raceresults_2 _index_2 (+ _index_2 1))))))

(event Custom|ShowTimer
  (bind _wbp_timer (Variables|Default|GetWBP_Timer))
  ;[0.15 0.15 0.15 0.5] タイマー表示
  (Utilities|IsValid _wbp_timer
    (:Is%20Valid
      (Widget|SetVisibility _wbp_timer "HitTestInvisible"))
    (:Is%20Not%20Valid
      (Development|PrintString 0 "WBP_Timer is Invalid!"))))

(fn TimespantoString
  (params (Time :type Timespan%20Structure))
  (bind (_days _hours _minutes _seconds _milliseconds) (Math|Timespan|BreakTimespan Time))
  (return (Utilities|String|Append (Utilities|String|ToString(Text) (Utilities|Text|ToText(Integer) _minutes false true 2)) " : " (Utilities|String|ToString(Text) (Utilities|Text|ToText(Integer) _seconds false true 2)) " : " (Utilities|String|ToString(Text) (Utilities|Text|ToText(Integer) _milliseconds false true 2)))))