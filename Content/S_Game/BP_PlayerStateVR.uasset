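; VR PlayerState that runs a two-race series, solo or multiplayer, from countdown to final ranking.
; RaceStart places the pawn through CourseManager and locks input during countdown; RaceEnd records time and returns it to practice.
; In multiplayer, the host registers test-named players with skins, and times are relayed to every PlayerState.
; Bubble sorts rank per-race and cumulative results for the widgets; timed delays and debug auto-start drive the flow.
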(event Custom|Race%20Start
  (bind _returnvalue (Game|Player|GetPlayerPawn 0))
  (bind _playercontroller (Variables|Default|GetPlayerController))
  (bind _asvrpawn (Utilities|Casting|CastToVRPawn _returnvalue))
  (bind _wbp_start (Variables|/Game/S_Game/BP_PlayerControllerVR.BP_PlayerControllerVR_C|GetWBP_Start _playercontroller))
  (bind _wbp_timer (Variables|/Game/S_Game/BP_PlayerControllerVR.BP_PlayerControllerVR_C|GetWBP_Timer _playercontroller))
  (bind _returnvalue_2 (UserInterface|GetWidget _wbp_start))
  (bind _returnvalue_3 (UserInterface|GetWidget _wbp_timer))
  (bind _aswbp_start (Utilities|Casting|CastToWBP_Start _returnvalue_2))
  (bind _aswbp_timer (Utilities|Casting|CastToWBP_Timer _returnvalue_3))
  (if (Variables|Default|GetisGoal) ; レース中は実行しない
    (if (Networking|IsServer)
      (if (Variables|Default|GetisSolo)
        ;[0.15 0.15 0.15 0.5] カウントダウンアニメーション分のタイム補正をかけて開始時間を保存
        (Variables|Default|SetRaceStartTime (+ (Math|DateTime|Now) (Math|Timespan|MakeTimespan 0 0 0 5)) :!label _label)
        (Variables|Default|SetisGoal false) ; ゴール受け付け開始
        (Default|RaceSetup (Variables|Default|GetCourseManager) (Variables|Default|GetRaceNumber)) ; コースの準備
        ;[0.15 0.15 0.15 0.5] 入力を無効化しながらスタート位置に移動
        (bind _startposition (Default|GetStartPosition (Variables|Default|GetCourseManager) (Variables|Default|GetRaceNumber) (Variables|Default|GetID)))
        (Class|VRPawn|SetPosition _asvrpawn _startposition)
        (Variables|/Script/VRTemplate.VRPawn|SetbEnableInpute _asvrpawn false)
        ;[0.15 0.15 0.15 0.5] UI有効化
        (Variables|/Game/K_Level/WBP_Timer.WBP_Timer_C|SetIsBlinking _aswbp_timer false)
        (Widget|SetVisibility _aswbp_timer "HitTestInvisible")
        (Default|PlaySE _aswbp_start)
        (UserInterface|Animation|PlayAnimation _aswbp_start (Variables|/Game/K_Level/WBP_Start.WBP_Start_C|GetStart _aswbp_start) 0.0 1 "Forward" 1.0 false)
        (Widget|SetVisibility _aswbp_start "Visible")
        ;[0.15 0.15 0.15 0.5] ゲーム開始と同時に入力を有効化
        (Utilities|FlowControl|Delay 5.0)
        (Variables|/Script/VRTemplate.VRPawn|SetbEnableInpute _asvrpawn true))
      (elif (Utilities|IsValid (Variables|Default|GetPlayerController))
        (goto _label)))))

(event Custom|Race%20End
  (bind _returnvalue (Math|DateTime|Now))
  (bind _racestarttime (Variables|Default|GetRaceStartTime))
  (bind _playercontroller (Variables|Default|GetPlayerController))
  (bind _raceresults (Variables|Default|GetRaceResults))
  (bind _raceresults_full (Variables|Default|GetRaceResults_Full))
  (bind _returnvalue_2 (- _returnvalue _racestarttime))
  (bind _output (Utilities|Array|Get(acopy) _raceresults_full))
  (bind _wbp_timer (Variables|/Game/S_Game/BP_PlayerControllerVR.BP_PlayerControllerVR_C|GetWBP_Timer _playercontroller))
  (bind _wbp_goal (Variables|/Game/S_Game/BP_PlayerControllerVR.BP_PlayerControllerVR_C|GetWBP_Goal _playercontroller))
  (bind _returnvalue_3 (UserInterface|GetWidget _wbp_timer))
  (bind _returnvalue_4 (UserInterface|GetWidget _wbp_goal))
  (bind _aswbp_timer (Utilities|Casting|CastToWBP_Timer _returnvalue_3))
  (bind _aswbp_goal (Utilities|Casting|CastToWBP_Goal _returnvalue_4))
  ;[0.15 0.15 0.15 0.5] 実行は1回のみ
  (if (not (Variables|Default|GetisGoal))
    (Variables|Default|SetisGoal true)
    (if (Variables|Default|GetisSolo)
      ;[0.15 0.15 0.15 0.5] ソロプレイ用レース結果作成
      (if (== (Variables|Default|GetRaceNumber) 1)
        (Utilities|Array|Clear _raceresults_full)
        (Utilities|Array|Add _raceresults_full (Utilities|Struct|MakeRaceResult "You" 0 "+00000000.00:00:00.000000000")))
      (Utilities|Struct|SetmembersinRaceResult _output (+ (.RaceTime (Utilities|Struct|BreakRaceResult _output)) _returnvalue_2))
      (Utilities|Array|Clear _raceresults)
      (Utilities|Array|Add _raceresults (Utilities|Struct|MakeRaceResult "You" 0 _returnvalue_2))
      (else
        ;[0.15 0.15 0.15 0.5] ローカルでタイムを計算し送信
        (CallFunction|SendRaceResult _returnvalue_2)))
    ;[0.15 0.15 0.15 0.5] ゴール時アニメーションなど
    (UserInterface|Animation|PlayAnimation _aswbp_goal (Variables|/Game/K_Level/WBP_Goal.WBP_Goal_C|GetGoal _aswbp_goal) 0.0 1 "Forward" 1.0 false)
    (Widget|SetVisibility _aswbp_goal "HitTestInvisible")
    (Default|StartBlinking _aswbp_timer)
    (Default|SetTime _aswbp_timer _returnvalue_2)
    ;[0.15 0.15 0.15 0.5] 練習エリアに戻す
    (bind _practiceposition (Default|GetPracticePosition (Variables|Default|GetCourseManager) (Variables|Default|GetID)))
    (Class|VRPawn|SetPosition (.AsVRPawn (Utilities|Casting|CastToVRPawn (Game|Player|GetPlayerPawn 0))) _practiceposition)
    ;[0.15 0.15 0.15 0.5] ソロプレイなら結果を表示
    (if (Variables|Default|GetisSolo)
      (Utilities|FlowControl|Delay 3.0)
      (CallFunction|DisplayRaceResult (Utilities|String|Append "第" (Utilities|String|ToString(Integer) (Variables|Default|GetRaceNumber)) "レースリザルト") (Variables|Default|GetRaceResults))
      (Utilities|FlowControl|Delay 7.0)
      (CallFunction|RemoveRaceResult)
      (Utilities|FlowControl|Delay 2.0)
      (switch int (Variables|Default|GetRaceNumber)
        (:1
          (Variables|Default|SetRaceNumber 2)
          (CallFunction|RaceStart))
        (:2
          (Variables|Default|SetRaceNumber 1)
          (CallFunction|MakeFullRaceRanking)
          (CallFunction|DisplayRaceResult "最終リザルト" (Variables|Default|GetRaceResults_Full)))))))

(event Custom|Make%20Race%20Ranking
  (bind _raceresults (Variables|Default|GetRaceResults))
  (bind _raceresults_2 (Variables|Default|GetRaceResults))
  (bind _returnvalue (Utilities|Array|Length _raceresults))
  ;[0.15 0.15 0.15 0.5] レース結果をタイム順に並べ替え
  (for _index (range 0 (- _returnvalue 1))
    (for _index_2 (range 0 (- _returnvalue 2))
      (if (> (.RaceTime (Utilities|Struct|BreakRaceResult (Utilities|Array|Get(acopy) _raceresults_2 _index_2))) (.RaceTime (Utilities|Struct|BreakRaceResult (Utilities|Array|Get(acopy) _raceresults_2 (+ _index_2 1)))))
        (Utilities|Array|Swap _raceresults_2 _index_2 (+ _index_2 1))))))

(event Custom|Display%20Race%20Result
  (params (ResultName :type String) (RaceResult :type Array%20of%20Race%20Result%20Structures))
  ;[0.15 0.15 0.15 0.5] レース結果表示
  (if (Networking|IsServer)
    (if (Variables|Default|GetisSolo)
      (Widget|SetVisibility (.AsWBP%20Timer (Utilities|Casting|CastToWBP_Timer (UserInterface|GetWidget (Variables|/Game/S_Game/BP_PlayerControllerVR.BP_PlayerControllerVR_C|GetWBP_Timer (Variables|Default|GetPlayerController))))) "Hidden" :!label _label)
      (Default|DisplayResult (.AsWBP%20Race%20Result (Utilities|Casting|CastToWBP_RaceResult (UserInterface|GetWidget (Variables|/Game/S_Game/BP_PlayerControllerVR.BP_PlayerControllerVR_C|GetWBP_RaceResult (Variables|Default|GetPlayerController))))) ResultName RaceResult))
    (else
      (goto _label))))

(event Custom|Send%20Race%20Result
  (params (RaceTime :type Timespan%20Structure))
  ;[0.15 0.15 0.15 0.5] クライアントからホストを経由して全ユーザーにレース結果（タイム）を送信
  (for _index (range 0 (- (Class|GameplayStatics|GetNumPlayerControllers) 1))
    (bind _asbp_player_state_vr (Utilities|Casting|CastToBP_PlayerStateVR (Variables|/Script/Engine.Controller|GetPlayerState (Game|GetPlayerController _index))))
    (CallFunction|MakeRaceResult _asbp_player_state_vr (Variables|Default|GetID) RaceTime)))

(event Custom|Save%20Race%20Results
  (for _array_element (Variables|Default|GetRaceResults)
    (Utilities|Array|Add (Variables|Default|GetPlayerResults) (Utilities|Struct|MakePlayerResult (.PlayerName (Utilities|Struct|BreakRaceResult _array_element)) (.RaceTime (Utilities|Struct|BreakRaceResult _array_element))))))

(event Custom|Register%20Player
  (params (SkinId :type Integer) (PlayerControllerIndex :type Integer) (PlayerName :type String))
  ;[0.15 0.15 0.15 0.5] ホスト側のスキン変更処理
  (bind _asvrpawn (Utilities|Casting|CastToVRPawn (Pawn|GetControlledPawn (Game|GetPlayerController PlayerControllerIndex))))
  (switch int SkinId
    (:Default
      (Class|VRPawn|ChangeBodyMaterial _asvrpawn "/Game/K_Level/Character/body.body" :!label _label))
    (:0
      (goto _label))
    (:1
      (Class|VRPawn|ChangeBodyMaterial _asvrpawn "/Game/K_Level/Character/body2.body2"))
    (:2
      (Class|VRPawn|ChangeBodyMaterial _asvrpawn "/Game/K_Level/Character/body3.body3"))
    (:3
      (Class|VRPawn|ChangeBodyMaterial _asvrpawn "/Game/K_Level/Character/body4.body4")))
  ;[0.15 0.15 0.15 0.5] 全ユーザーに登録プレイヤーの情報共有
  (for _index (range 0 (- (Class|GameplayStatics|GetNumPlayerControllers) 1))
    (bind _asbp_player_state_vr (Utilities|Casting|CastToBP_PlayerStateVR (Variables|/Script/Engine.Controller|GetPlayerState (Game|GetPlayerController _index))))
    (CallFunction|RegisterUnlocal _asbp_player_state_vr PlayerControllerIndex PlayerName)
    ;[0.15 0.15 0.15 0.5] IDを該当者本人に教える
    (if (== _index PlayerControllerIndex)
      (Variables|BP_PlayerStateVR_C|SetID _asbp_player_state_vr PlayerControllerIndex))))

(event Custom|Remove%20Race%20Result
  (bind _playercontroller (Variables|Default|GetPlayerController))
  (bind _wbp_raceresult (Variables|/Game/S_Game/BP_PlayerControllerVR.BP_PlayerControllerVR_C|GetWBP_RaceResult _playercontroller))
  (bind _returnvalue (UserInterface|GetWidget _wbp_raceresult))
  (bind _aswbp_race_result (Utilities|Casting|CastToWBP_RaceResult _returnvalue))
  ;[0.15 0.15 0.15 0.5] レース結果非表示
  (if (Networking|IsServer)
    (if (Variables|Default|GetisSolo)
      (UserInterface|Animation|PlayAnimation _aswbp_race_result (Variables|/Game/K_Level/WBP_RaceResult.WBP_RaceResult_C|GetRemove _aswbp_race_result) 0.0 1 "Forward" 1.0 false :!label _label))
    (else
      (goto _label))))

(event Custom|Make%20Full%20Race%20Ranking
  (bind _raceresults_full (Variables|Default|GetRaceResults_Full))
  (bind _raceresults_full_2 (Variables|Default|GetRaceResults_Full))
  (bind _returnvalue (Utilities|Array|Length _raceresults_full))
  ;[0.15 0.15 0.15 0.5] レース結果をタイム順に並べ替え
  (for _index (range 0 (- _returnvalue 1))
    (for _index_2 (range 0 (- _returnvalue 2))
      (if (> (.RaceTime (Utilities|Struct|BreakRaceResult (Utilities|Array|Get(acopy) _raceresults_full_2 _index_2))) (.RaceTime (Utilities|Struct|BreakRaceResult (Utilities|Array|Get(acopy) _raceresults_full_2 (+ _index_2 1)))))
        (Utilities|Array|Swap _raceresults_full_2 _index_2 (+ _index_2 1))))))

(event Custom|ResetRaceData
  ;[0.15 0.15 0.15 0.5] リセット処理
  (Utilities|Array|Clear (Variables|Default|GetRaceResults))
  (Variables|Default|SetGoalCount 0)
  (Variables|Default|SetRaceNumber 1))

(event Custom|Register%20Unlocal
  (params (PlayerControllerIndex :type Integer) (PlayerName :type String))
  (bind _raceresult (Utilities|Struct|MakeRaceResult PlayerName PlayerControllerIndex "+00000000.00:00:00.000000000"))
  ;[0.15 0.15 0.15 0.5] ホスト側にあるPlayerStateにレースプレイヤーの登録
  (if (> (Class|GameplayStatics|GetNumPlayerControllers) PlayerControllerIndex)
    (Utilities|Array|Add (Variables|Default|GetRaceResults) _raceresult)
    (Utilities|Array|Add (Variables|Default|GetRaceResults_Full) _raceresult)))

(event Custom|Make%20Race%20Result
  (params (PlayerID :type Integer) (RaceTime :type Timespan%20Structure))
  (bind _raceresults (Variables|Default|GetRaceResults))
  ;[0.15 0.15 0.15 0.5] レース結果集計
  (bind (_array_element _array_index) (Utilities|Array|ForEachLoopwithBreak _raceresults :!label _label)
    (:LoopBody
      (if (== (.PlayerId (Utilities|Struct|BreakRaceResult _array_element)) PlayerID)
        (Utilities|Struct|SetmembersinRaceResult (Utilities|Array|Get(acopy) _raceresults _array_index) RaceTime)
        (Utilities|Struct|SetmembersinRaceResult (Utilities|Array|Get(acopy) (Variables|Default|GetRaceResults_Full) _array_index) (+ RaceTime (.RaceTime (Utilities|Struct|BreakRaceResult (Utilities|Array|Get(acopy) (Variables|Default|GetRaceResults_Full) _array_index)))))
        (bind _result (Math|Integer|IncrementInt (Variables|Default|GetGoalCount))
          (:%20%20
            (Variables|Default|SetGoalCount _result)
            (goto _label Break)))))
    (:Completed
      ;[0.15 0.15 0.15 0.5] 全員がゴールした場合（共通処理）
      (if (== (Variables|Default|GetGoalCount) (Utilities|Array|Length _raceresults))
        (CallFunction|MakeRaceRanking)
        (Utilities|FlowControl|Delay 3.0) ; 最後の人のゴール演出待ち
        (CallFunction|DisplayRaceResult (Utilities|String|Append "第" (Utilities|String|ToString(Integer) (Variables|Default|GetRaceNumber)) "レースリザルト") (Variables|Default|GetRaceResults))
        (Utilities|FlowControl|Delay 7.0)
        (CallFunction|RemoveRaceResult)
        (Utilities|FlowControl|Delay 2.0)
        (switch int (Variables|Default|GetRaceNumber)
          (:Default
            (Variables|Default|SetRaceNumber 1 :!label _label_2))
          (:0
            (goto _label_2))
          (:1
            (Variables|Default|SetRaceNumber 2)
            (Variables|Default|SetGoalCount 0)
            (CallFunction|RaceStart))
          (:2
            (Variables|Default|SetRaceNumber 1)
            (CallFunction|MakeFullRaceRanking)
            (CallFunction|DisplayRaceResult "最終リザルト" (Variables|Default|GetRaceResults_Full))))))))

(event EventBeginPlay
  (CallFunction|ResetRaceData)
  (Variables|Default|SetPlayerController (.AsBP%20Player%20Controller%20VR (Utilities|Casting|CastToBP_PlayerControllerVR (Components|GetOwner))))
  (bind _output_get (Variables|Default|SetisSolo (Variables|/Game/G_Game/BP_GameInstance.BP_GameInstance_C|GetisSolo (.AsBP%20Game%20Instance (Utilities|Casting|CastToBP_GameInstance (Game|GetGameInstance))))))
  (if _output_get
    (Variables|Default|SetID 1)
    ;[0.15 0.15 0.15 0.5] デバッグ用
    (Utilities|FlowControl|Delay 1e+01)
    (CallFunction|RaceStart)
    (elif (Networking|IsServer)
      (if (Pawn|IsLocalPlayerController (Variables|Default|GetPlayerController))
        (Utilities|FlowControl|Delay 3.0)
        (for _index (range 1 (- (Class|GameplayStatics|GetNumPlayerControllers) 1))
          (CallFunction|RegisterPlayer (+ _index 0) _index (Utilities|String|Append "Test" (Utilities|String|ToString(Integer) _index))))
        (else
          (Utilities|FlowControl|Delay 5.0)
          (CallFunction|RaceStart))))))

(fn ConstructionScript)

(fn SaveRaceResult)