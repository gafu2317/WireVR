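; VR player controller for a race game that owns the race HUD and relays player IDs.
; On non-server BeginPlay, it waits a second for PlayerState to settle, then creates and stores start, goal, result and timer widgets.
; The host event looks up the controller indexed by device ID and forwards the player ID, which the client event writes to BP_PlayerStateVR.
; StopTimer makes the timer widget blink.
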(event Custom|Set%20PlayerId_Client
  (params (PlayerId :type Integer))
  (bind _asbp_player_state_vr (Utilities|Casting|CastToBP_PlayerStateVR (Game|GetPlayerState 0)))
  (Variables|/Game/S_Game/BP_PlayerStateVR.BP_PlayerStateVR_C|SetID _asbp_player_state_vr PlayerId))

(event Custom|Set%20PlayerId_Host
  (params (DeviceId :type Integer) (Player%20Id :type Integer))
  (bind _asbp_player_controller_vr (Utilities|Casting|CastToBP_PlayerControllerVR (Game|GetPlayerController DeviceId)))
  (CallFunction|SetPlayerIdClient _asbp_player_controller_vr Player%20Id))

(event Custom|StopTimer
  (bind _wbp_timer (Variables|Default|GetWBP_Timer))
  (Utilities|IsValid _wbp_timer
    (:Is%20Valid
      (Default|StartBlinking _wbp_timer))))

(event EventBeginPlay
  (if (not (Networking|IsServer))
    (Utilities|FlowControl|Delay 1.0) ; PlayerStateが落ち着くまで待機
    ;[0.15 0.15 0.15 0.5] WBP_Startの作成と変数格納
    (bind _returnvalue (UserInterface|CreateWidget "/Game/K_Level/WBP_Start.WBP_Start_C" self))
    (UserInterface|Viewport|AddtoViewport _returnvalue 0)
    (Variables|Default|SetWBP_Start _returnvalue)
    ;[0.15 0.15 0.15 0.5] WBP_Goalの作成と変数格納
    (bind _returnvalue_2 (UserInterface|CreateWidget "/Game/K_Level/WBP_Goal.WBP_Goal_C" self))
    (UserInterface|Viewport|AddtoViewport _returnvalue_2 0)
    (Variables|Default|SetWBP_Goal _returnvalue_2)
    ;[0.15 0.15 0.15 0.5] WBP_RaceResultの作成と変数格納
    (bind _returnvalue_3 (UserInterface|CreateWidget "/Game/K_Level/WBP_RaceResult.WBP_RaceResult_C" self))
    (UserInterface|Viewport|AddtoViewport _returnvalue_3 0)
    (Variables|Default|SetWBP_RaceResult _returnvalue_3)
    ;[0.15 0.15 0.15 0.5] WBP_Timerの作成
    (bind _returnvalue_4 (UserInterface|CreateWidget "/Game/K_Level/WBP_Timer.WBP_Timer_C" self))
    (bind _output_get (Variables|Default|SetWBP_Timer _returnvalue_4))
    (UserInterface|Viewport|AddtoViewport _output_get 0)))

(fn ConstructionScript)